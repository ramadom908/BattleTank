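; Player-controlled tank pawn that wires up its aiming, movement and health bar components and routes player input to them.
; On BeginPlay it gives TankAiming the player projectile, barrel and turret, gives TankMovement both tracks, and links the HealthBar widget to itself.
; Input drives movement and firing through those components, rotates the azimuth gimbal and spring arm with frame-time scaling, and toggles between the main and first-person cameras.
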(event `self.ReceiveBeginPlay`
  (set `TankAimingComponent.ProjectileBlueprint` "/Game/Projectile/Projectile_BP2_Player.Projectile_BP2_Player_C" (`self.TankAiming`))
  (`TankAimingComponent.Initialise` (`self.TankAiming`) (`self.TankBarrel`) (`self.TankTurret`))
  (`TankMovementComponent.Initialise` (`self.TankMovement`) (`self.TankTrack`) (`self.RightTrack`))
  (`self.InitializeHealthWidge2`))

(event `InputAction|SwapCam`
  (params (Key :type "Key Structure"))
  (:`Pressed`
    (`ActorComponent.ToggleActive` (`self.Camera2FirstPerson`))
    (`ActorComponent.ToggleActive` (`self.Camera`))))

(event `InputAxis|AimAzimuth`
  (params (AxisValue :type "Float (single-precision)"))
  (`SceneComponent.K2_AddLocalRotation` (`self.AzimuthGimbal`) (`KismetMathLibrary.MakeRotator` 0.0 0.0 (* AxisValue (`GameplayStatics.GetWorldDeltaSeconds`) 100.0)) false false))

(event `InputAxis|MoveForward`
  (params (AxisValue :type "Float (single-precision)"))
  (`TankMovementComponent.IntendMoveForward` (`self.TankMovement`) AxisValue))

(event `InputAxis|AimElevation`
  (params (AxisValue :type "Float (single-precision)"))
  (`SceneComponent.K2_AddLocalRotation` (`self.SpringArm`) (`KismetMathLibrary.MakeRotator` 0.0 (* AxisValue (`GameplayStatics.GetWorldDeltaSeconds`) 100.0)) false false))

(event `InputAxis|Turn Right`
  (params (AxisValue :type "Float (single-precision)"))
  (`TankMovementComponent.IntendTurnRight` (`self.TankMovement`) AxisValue))

(event `InputAction|Fire99`
  (params (Key :type "Key Structure"))
  (:`Pressed`
    (`TankAimingComponent.Fire` (`self.TankAiming`))))

(fn `InitializeHealthWidge2`
  (bind _ashealth_bar (cast `/Game/UI/HealthBar` (`WidgetComponent.GetUserWidgetObject` (`self.Widget`))))
  (set `/Game/UI/HealthBar.MyTank` self _ashealth_bar))

(fn `InitializeHealthwidget`
  (bind _ashealth_bar (cast `/Game/UI/HealthBar` (`WidgetComponent.GetUserWidgetObject` (`self.Widget`))))
  (set `/Game/UI/HealthBar.MyTank` null _ashealth_bar))

(fn `UserConstructionScript`)