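; Player-controllable tank pawn Blueprint that wires input and components to tank logic.
; On BeginPlay it passes its barrel and turret components to inherited setter functions.
; Aim axes rotate an azimuth gimbal and the spring arm, scaled by frame delta time, to orbit the camera.
; Separate axes set left and right track throttle for differential steering, and a fire action calls Fire.
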(event `self.ReceiveBeginPlay`
  (`self.SetBarrelReference` (`self.TankBarrel`))
  (`self.SetTurretReference` (`self.TankTurret`)))

(event `InputAxis|AimAzimuth`
  (params (AxisValue :type "Float (single-precision)"))
  (`SceneComponent.K2_AddLocalRotation` (`self.AzimuthGimbal`) (`KismetMathLibrary.MakeRotator` 0.0 0.0 (* AxisValue (`GameplayStatics.GetWorldDeltaSeconds`) 100.0)) false false))

(event `InputAxis|AimElevation`
  (params (AxisValue :type "Float (single-precision)"))
  (`SceneComponent.K2_AddLocalRotation` (`self.SpringArm`) (`KismetMathLibrary.MakeRotator` 0.0 (* AxisValue (`GameplayStatics.GetWorldDeltaSeconds`) 100.0)) false false))

(event `InputAction|Fire99`
  (params (Key :type "Key Structure"))
  (:`Pressed`
    (`self.Fire`)))

(event `InputAction|LeftTrackForward`
  (params (Key :type "Key Structure")))

(event `InputAction|RightTrackForward`
  (params (Key :type "Key Structure")))

(event `InputAxis|AxisLeftTrackForward`
  (params (AxisValue :type "Float (single-precision)"))
  (`TankTrack.SetThrottle` (`self.LeftTankTrack`) AxisValue))

(event `InputAxis|AxisRightTrackForward`
  (params (AxisValue :type "Float (single-precision)"))
  (`TankTrack.SetThrottle` (`self.RightTankTrack`) AxisValue))

(fn `UserConstructionScript`)